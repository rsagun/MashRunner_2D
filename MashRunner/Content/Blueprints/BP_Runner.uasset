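; BP_Runner is a flipbook-sprite character that runs along +X, powered by alternating left and right taps.
; BeginPlay adds the Enhanced Input mapping; each tap differing from the last raises MaxWalkSpeed.
; Tick applies constant forward input while decaying that speed toward zero, frame-rate independently.
; Velocity selects the idle or run flipbook and scales run playback relative to MaxSpeed.
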(event `self.ReceiveBeginPlay`
  ;[1 1 1] Register player controller and mapping context
  (bind _asplayer_controller (cast `PlayerController` (`self.GetController`)))
  (`EnhancedInputSubsystemInterface.AddMappingContext` (pcsubsystem `EnhancedInputLocalPlayerSubsystem` _asplayer_controller) "/Game/Input/IMC_Runner.IMC_Runner" 0 (struct)))

(event `self.ReceiveTick`
  (params (DeltaSeconds :type "Float (single-precision)"))
  (bind _charactermovement (`self.CharacterMovement`))
  (bind _sprite (`self.Sprite`))
  (bind _returnvalue (`KismetMathLibrary.VSize` (`MovementComponent.Velocity` (`self.CharacterMovement`))))
  (`self.AddMovementInput` (1.0 0.0 0.0))
  (set `CharacterMovementComponent.MaxWalkSpeed` (`KismetMathLibrary.FMax` 0.0 (- (`CharacterMovementComponent.MaxWalkSpeed` _charactermovement) (* (`self.RunSpeedReducedPerDeltaTime`) DeltaSeconds))) _charactermovement)
  ;[1 1 1] Based on the players velocity, update flipbook animation played (idle or run).
  (`PaperFlipbookComponent.SetFlipbook` _sprite (select `bool` (> _returnvalue 0.0) :`false` "/Game/PaperAssets/Runner/FB_Runner_Idle.FB_Runner_Idle" :`true` "/Game/PaperAssets/Runner/FB_Runner_Run.FB_Runner_Run" :!type "PaperFlipbook Object Reference"))
  ;[1 1 1] Player velocity > 0, adjust play rate of animation proportionate to speed. Player velocity <= 0, set play rate to default of 1 for idle animation.
  (if (== (`PaperFlipbookComponent.GetFlipbook` _sprite) "/Game/PaperAssets/Runner/FB_Runner_Run.FB_Runner_Run")
    (`PaperFlipbookComponent.SetPlayRate` _sprite (/ _returnvalue (`self.MaxSpeed`)))
    (else
      (`PaperFlipbookComponent.SetPlayRate` _sprite 1.0))))

(event `EnhancedInput|/Game/Input/Actions/IA_PowerLeft`
  (params (ActionValue :type Boolean) (ElapsedSeconds :type "Float (double-precision)") (TriggeredSeconds :type "Float (double-precision)") (InputAction :type "InputAction Object Reference" :default "/Game/Input/Actions/IA_PowerLeft.IA_PowerLeft"))
  ;[1 1 1] Increase speed based on alternating inputs (a - d/left - right)
  (:`Started`
    (if (`|EnumInequality` (`self.LastInput`) "NewEnumerator1")
      (set `self.LastInput` "NewEnumerator1")
      (`self.Increase Run Speed`))))

(event `EnhancedInput|/Game/Input/Actions/IA_PowerRight`
  (params (ActionValue :type Boolean) (ElapsedSeconds :type "Float (double-precision)") (TriggeredSeconds :type "Float (double-precision)") (InputAction :type "InputAction Object Reference" :default "/Game/Input/Actions/IA_PowerRight.IA_PowerRight"))
  ;[1 1 1] Increase speed based on alternating inputs (a - d/left - right)
  (:`Started`
    (if (`|EnumInequality` (`self.LastInput`) "NewEnumerator2")
      (set `self.LastInput` "NewEnumerator2")
      (`self.Increase Run Speed`))))

(fn `Increase Run Speed`
  (bind _charactermovement (`self.CharacterMovement`))
  (set `CharacterMovementComponent.MaxWalkSpeed` (+ (`CharacterMovementComponent.MaxWalkSpeed` _charactermovement) (`self.RunSpeedPerTap`)) _charactermovement))

(fn `UserConstructionScript`)